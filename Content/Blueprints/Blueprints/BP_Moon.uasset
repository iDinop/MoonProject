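; BP_Moon is a puzzle moon that lights BP_MoonlightReceiver actors with traced moonlight, or slides its sphere in gravity-puzzle mode.
; Outside that mode, a looping timer fires a center ray plus concentric cone rings of debug-drawn traces, toggling receivers through sensor hits.
; StateSwitch uses timelines to step through preset pitches or, in gravity mode, positions; all three states behave identically.
; BeginPlay registers the moon with the player and receivers.
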(event Custom|StateSwitch
  ;[0.15 0.15 0.15 0.5 74] State Check event
  (if (Variables|Booleans|GetisState1)
    (if (Variables|Booleans|GetbGravityPuzzle)
      (CallFunction|MoveMoon)
      (else
        (CallFunction|RotateMoon)
        (CallFunction|UpdateLightDirection)))
    (elif (Variables|Booleans|GetisState2)
      (if (Variables|Booleans|GetbGravityPuzzle)
        (CallFunction|MoveMoon)
        (else
          (CallFunction|RotateMoon)
          (CallFunction|UpdateLightDirection)))
      (elif (Variables|Booleans|GetisState3)
        (if (Variables|Booleans|GetbGravityPuzzle)
          (CallFunction|MoveMoon)
          (else
            (CallFunction|RotateMoon)
            (CallFunction|UpdateLightDirection)))
        (else
          (Development|PrintString "no state on"))))))

(event Custom|UpdateLightDirection
  ;[0.15 0.15 0.15 0.5 74] Update Light Direction event
  (Variables|Vectors|SetLightForward "0, 0, 0")
  (Variables|Vectors|SetRayDir (Math|Vector|NegateVector (Variables|Vectors|GetLightForward))))

(event Custom|RotateMoon
  (bind _degreesarray (Variables|Floats|GetDegreesArray))
  ;[0.15 0.15 0.15 0.5 74] Set Moon Rotation
  (if (not (Variables|Booleans|GetisRotating))
    (Variables|Booleans|SetisRotating true)
    (Variables|Floats|SetStartPitch (Utilities|Array|Get(acopy) _degreesarray (Variables|Integers|GetCurrentStep)))
    (Variables|Integers|SetCurrentStep (Math|Integer|%(Integer) (+ (Variables|Integers|GetCurrentStep) 1) (Utilities|Array|Length _degreesarray)))
    (Variables|Floats|SetTargetPitch (Utilities|Array|Get(acopy) (Variables|Floats|GetDegreesArray) (Variables|Integers|GetCurrentStep)))
    (bind _moonrotation (Timeline|MoonRotation PlayFromStart)
      (:Update
        (Transformation|SetActorRotation (Math|Rotator|MakeRotator 0.0 (Math|Float|Lerp (Variables|Floats|GetStartPitch) (Variables|Floats|GetTargetPitch) _moonrotation) 0.0)))
      (:Finished
        (Variables|Booleans|SetisRotating false)))))

(event Custom|FireSingleRay
  (bind _rayorigin (Variables|Default|GetRayOrigin))
  (bind _returnvalue (Transformation|GetWorldLocation _rayorigin))
  ;[0.15 0.15 0.15 0.5 74] Fire Single Ray Event
  (bind (_outhit _returnvalue_2) (Collision|LineTraceByChannel _returnvalue (+ _returnvalue (* (Math|Vector|Normalize (Math|Vector|SelectVector (Variables|Vectors|GetRayDirection) (Math|Vector|NegateVector (Math|Vector|GetForwardVector _rayorigin)) (Variables|Booleans|GetbUseCustomRayDirection))) (Variables|Floats|GetTraceDistance))) "TraceTypeQuery1" false 0 "ForDuration"))
  (if _returnvalue_2
    (bind _asbp_moonlight_receiver (Utilities|Casting|CastToBP_MoonlightReceiver (.HitActor (Collision|BreakHitResult _outhit))))
    (if (== (Variables|/Game/Blueprints/Blueprints/BP_MoonlightReceiver.BP_MoonlightReceiver_C|GetSensor _asbp_moonlight_receiver) (.HitComponent (Collision|BreakHitResult _outhit)))
      (Variables|Booleans|SetbAnyReceiverHitThisTick true)
      (Variables|Actors|SetReceiverHitThisTick _asbp_moonlight_receiver)
      (bind _output_get (Variables|Actors|SetCurrentHitReceiver _asbp_moonlight_receiver))
      (if (!= (Variables|Actors|GetLastHitReceiver) _output_get)
        (Utilities|IsValid (Variables|Actors|GetLastHitReceiver)
          (:Is%20Valid
            (Default|SetLit (Variables|Actors|GetLastHitReceiver) false)
            (Default|SetLit (Variables|Actors|GetCurrentHitReceiver) true)
            (Variables|Actors|SetLastHitReceiver (Variables|Actors|GetCurrentHitReceiver)))
          (:Is%20Not%20Valid
            (Default|SetLit (Variables|Actors|GetCurrentHitReceiver) true)
            (Variables|Actors|SetLastHitReceiver (Variables|Actors|GetCurrentHitReceiver)))))
      (else
        (Utilities|IsValid (Variables|Actors|GetLastHitReceiver) :!label _label
          (:Is%20Valid
            (Default|SetLit (Variables|Actors|GetLastHitReceiver) false)
            (Variables|Actors|SetLastHitReceiver 0)))))
    (else
      (goto _label))))

(event Custom|MoveMoon
  (bind _positionsarray (Variables|Floats|GetPositionsArray))
  ;[0.15 0.15 0.15 0.5 74] Set Moon Position
  (if (not (Variables|Booleans|GetbIsMoving))
    (Variables|Booleans|SetbIsMoving true)
    (Variables|Floats|SetStartPosition (Utilities|Array|Get(acopy) _positionsarray (Variables|Integers|GetCurrentStep)))
    (Variables|Integers|SetCurrentStep (Math|Integer|%(Integer) (+ (Variables|Integers|GetCurrentStep) 1) (Utilities|Array|Length _positionsarray)))
    (Variables|Floats|SetEndPosition (Utilities|Array|Get(acopy) (Variables|Floats|GetPositionsArray) (Variables|Integers|GetCurrentStep)))
    (bind _moonmovement (Timeline|MoonMovement PlayFromStart)
      (:Update
        (Transformation|SetRelativeLocation (Variables|Default|GetSphere) (Math|Vector|MakeVector (Math|Float|Lerp (Variables|Floats|GetStartPosition) (Variables|Floats|GetEndPosition) _moonmovement) 0.0 0.0) false false))
      (:Finished
        (Variables|Booleans|SetbIsMoving false)))))

(event Custom|FireConeRays
  (bind _returnvalue (Math|Vector|MakeVector 0.0 0.0 1.0))
  (bind _rings (Variables|Integers|GetRings))
  ;[0.15 0.15 0.15 0.5 74] FireConeRays
  (if (not (Variables|Booleans|GetbGravityPuzzle))
    (bind _output_get (Variables|Vectors|SetBaseDir (Math|Vector|Normalize (Math|Vector|NegateVector (Math|Vector|GetForwardVector (Variables|Default|GetRayOrigin))))))
    (Variables|Booleans|SetbAnyReceiverHitThisTick false)
    (Variables|Actors|SetReceiverHitThisTick 0)
    (Variables|Booleans|SetbUseCustomRayDirection true)
    (Variables|Vectors|SetRayDirection _output_get)
    (CallFunction|FireSingleRay)
    (Variables|Vectors|SetUpRef (Math|Vector|SelectVector _returnvalue (Math|Vector|MakeVector 0.0 1.0 0.0) (< (Math|Float|Absolute(Float) (Math|Vector|DotProduct (Variables|Vectors|GetBaseDir) _returnvalue)) 0.95)))
    (Variables|Vectors|SetAxisA (Math|Vector|Normalize (Math|Vector|CrossProduct (Variables|Vectors|GetUpRef) (Variables|Vectors|GetBaseDir))))
    (Variables|Vectors|SetAxisB (Math|Vector|Normalize (Math|Vector|CrossProduct (Variables|Vectors|GetBaseDir) (Variables|Vectors|GetAxisA))))
    (for _index (range 0 (- _rings 1))
      (bind _output_get_2 (Variables|Integers|SetRingIndex _index))
      (bind _output_get_3 (Variables|Floats|SetRingT (/ (+ _output_get_2 1) (Math|Conversions|ToFloat(Integer) _rings))))
      (bind _output_get_4 (Variables|Floats|SetRingAngle (* (Variables|Floats|GetConeAngleDeg) _output_get_3)))
      (Variables|Floats|SetRingRad (Math|Trig|DegreesToRadians _output_get_4))
      (bind _output_get_5 (Variables|Floats|SetYawStepDeg (Math|Conversions|ToFloat(Integer) (/ 360 (Variables|Integers|GetRayCountPerRing)))))
      (for _index_2 (range 0 (- (Variables|Integers|GetRayCountPerRing) 1))
        (Variables|Integers|SetRayIndex _index_2)
        (bind _output_get_6 (Variables|Floats|SetYawDeg (* (Variables|Integers|GetRayIndex) _output_get_5)))
        (bind _output_get_7 (Variables|Floats|SetYawRad (Math|Trig|DegreesToRadians _output_get_6)))
        (Variables|Vectors|SetCircleDir (+ (* (Variables|Vectors|GetAxisA) (Math|Trig|Cos(Radians) _output_get_7)) (* (Variables|Vectors|GetAxisB) (Math|Trig|Sin(Radians) _output_get_7))))
        (bind _output_get_8 (Variables|Vectors|SetConeDir (Math|Vector|Normalize (+ (* (Variables|Vectors|GetBaseDir) (Math|Trig|Cos(Radians) (Variables|Floats|GetRingRad))) (* (Variables|Vectors|GetCircleDir) (Math|Trig|Sin(Radians) (Variables|Floats|GetRingRad)))))))
        (Variables|Booleans|SetbUseCustomRayDirection true)
        (Variables|Vectors|SetRayDirection _output_get_8)
        (CallFunction|FireSingleRay))
      (Variables|Booleans|SetbUseCustomRayDirection false)
      (if (Variables|Booleans|GetbAnyReceiverHitThisTick)
        (Default|SetLit (Variables|Actors|GetReceiverHitThisTick) true)
        (Variables|Actors|SetLastHitReceiver (Variables|Actors|GetReceiverHitThisTick))
        (else
          (Utilities|IsValid (Variables|Actors|GetLastHitReceiver)
            (:Is%20Valid
              (Default|SetLit (Variables|Actors|GetLastHitReceiver) false))
            (:Is%20Not%20Valid
              (Variables|Actors|SetLastHitReceiver 0))))))
    (Variables|Booleans|SetbUseCustomRayDirection false)))

(event EventBeginPlay
  ;[0.15 0.15 0.15 0.5 74] Begin Play
  (bind _asbp_first_person_character (Utilities|Casting|CastToBP_FirstPersonCharacter (Game|GetPlayerCharacter 0)))
  (bind _output_get (Variables|Character|SetPlayerRef _asbp_first_person_character))
  (Variables|/Game/FirstPerson/Blueprints/BP_FirstPersonCharacter.BP_FirstPersonCharacter_C|SetMoonREF_Debug _output_get self)
  (CallFunction|UpdateLightDirection)
  (for _array_element (Variables|Actors|GetReceiverREFS)
    (Variables|/Game/Blueprints/Blueprints/BP_MoonlightReceiver.BP_MoonlightReceiver_C|SetMoonREF _array_element self))
  (Development|PrintString "ReceiverREFs set")
  (Utilities|Time|SetTimerbyEvent (delegate Custom|FireConeRays) (Variables|Floats|GetCheckInterval) true))

(fn ConstructionScript)