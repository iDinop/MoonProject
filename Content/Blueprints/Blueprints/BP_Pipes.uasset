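; Interactable pipe actor that turns its static mesh a quarter turn each time it is interacted with.
; Interact stores the current relative rotation, combines it with a 90-degree yaw for the target, and plays the PipeRotation timeline to lerp between them along the shortest path.
; An IsRotating flag ignores further interactions until the timeline finishes.
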(event EventBeginPlay
  (bind _staticmesh (Variables|Default|GetStaticMesh))
  (bind _relativerotation (Variables|/Script/Engine.SceneComponent|GetRelativeRotation _staticmesh))
  (|CallParentFunction)
  (Variables|Rotators|SetBaseRotation (Math|Rotator|MakeRotator (.roll _relativerotation) (.pitch _relativerotation) 0.0)))

(event Collision|EventActorBeginOverlap
  (params (OtherActor :type Actor%20Object%20Reference)))

(event EventTick
  (params (DeltaSeconds :type Float%20%28single-precision%29)))

(event EventInteract
  (bind _staticmesh (Variables|Default|GetStaticMesh))
  (bind _relativerotation (Variables|/Script/Engine.SceneComponent|GetRelativeRotation _staticmesh))
  (if (not (Variables|Booleans|GetbIsRotating))
    (Variables|Booleans|SetbIsRotating true)
    (Variables|Rotators|SetBaseRotation _relativerotation)
    (Variables|Rotators|SetEndRotation (Math|Rotator|CombineRotators _relativerotation (Math|Rotator|MakeRotator 0.0 0.0 9e+01)))
    (bind _piperotation (Timeline|PipeRotation PlayFromStart)
      (:Update
        (Transformation|SetRelativeRotation (Variables|Default|GetStaticMesh) (Math|Rotator|Lerp(Rotator) (Variables|Rotators|GetBaseRotation) (Variables|Rotators|GetEndRotation) _piperotation true) false false))
      (:Finished
        (Variables|Booleans|SetbIsRotating false)))))

(fn ConstructionScript
  (|CallParentFunction))