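; BP_Activatable is an activatable object that triggers once all of its linked energy sources are fully charged.
; A looping timer started on BeginPlay polls the EnergySources array at CheckInterval and calls Activate when none is short of full charge.
; The timer is never cleared here, so Activate is called again on every check while the sources remain charged.
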(event Custom|CheckSources
  ;[0.15 0.15 0.15 0.5 74] Check Energy Sources Event
  (bind _allfullycharged (CallFunction|CheckSourcesCharge))
  (if _allfullycharged
    (CallFunction|Activate)))

(event EventBeginPlay
  ;[0.15 0.15 0.15 0.5 74] Begin Play
  (Utilities|Time|SetTimerbyEvent (delegate Custom|CheckSources) (Variables|Floats|GetCheckInterval) true))

(fn ConstructionScript)

(fn CheckSourcesCharge
  (for _array_element (Variables|Actors|GetEnergySources)
    (if (not (Variables|/Game/Blueprints/Blueprints/BP_MoonlightReceiver.BP_MoonlightReceiver_C|GetbIsFullyCharged _array_element))
      (return false)))
  (return true))