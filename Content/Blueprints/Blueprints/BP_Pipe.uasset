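; BP_Pipe is an interactable pipe piece with three connection colliders (bottom, left, right).
; Interact turns the mesh a quarter turn in yaw through a timeline-driven rotator lerp, ignoring input until it finishes.
; Each collider's overlap handler casts to another pipe and only prints debug connection text.
; Those checks compare the pipe's own overlapped component to the other pipe's colliders, rather than the other component.
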(event OnComponentBeginOverlap(CollisionBottom)
  (params (OverlappedComponent :type Primitive%20Component%20Object%20Reference) (OtherActor :type Actor%20Object%20Reference) (OtherComp :type Primitive%20Component%20Object%20Reference) (OtherBodyIndex :type Integer) (bFromSweep :type Boolean) (SweepResult :type Hit%20Result%20Structure%20%28by%20ref%29))
  (bind _asbp_pipe (Utilities|Casting|CastToBP_Pipe OtherActor))
  (if (== OverlappedComponent (Variables|BP_Pipe_C|GetCollisionRight _asbp_pipe))
    (Development|PrintString "Bottom connected to Right")
    (elif (== OverlappedComponent (Variables|BP_Pipe_C|GetCollisionLeft _asbp_pipe))
      (Development|PrintString "Bottom connected to Left")
      (elif (== OverlappedComponent (Variables|BP_Pipe_C|GetCollisionBottom _asbp_pipe))
        (Development|PrintString "Bottom connected to Bottom")))))

(event OnComponentBeginOverlap(CollisionRight)
  (params (OverlappedComponent :type Primitive%20Component%20Object%20Reference) (OtherActor :type Actor%20Object%20Reference) (OtherComp :type Primitive%20Component%20Object%20Reference) (OtherBodyIndex :type Integer) (bFromSweep :type Boolean) (SweepResult :type Hit%20Result%20Structure%20%28by%20ref%29))
  (bind _asbp_pipe (Utilities|Casting|CastToBP_Pipe OtherActor))
  (if (== OverlappedComponent (Variables|BP_Pipe_C|GetCollisionRight _asbp_pipe))
    (Development|PrintString "Right connected to Right")
    (elif (== OverlappedComponent (Variables|BP_Pipe_C|GetCollisionLeft _asbp_pipe))
      (Development|PrintString "Right connected to Left")
      (elif (== OverlappedComponent (Variables|BP_Pipe_C|GetCollisionBottom _asbp_pipe))
        (Development|PrintString "Right connected to Bottom")))))

(event OnComponentBeginOverlap(CollisionLeft)
  (params (OverlappedComponent :type Primitive%20Component%20Object%20Reference) (OtherActor :type Actor%20Object%20Reference) (OtherComp :type Primitive%20Component%20Object%20Reference) (OtherBodyIndex :type Integer) (bFromSweep :type Boolean) (SweepResult :type Hit%20Result%20Structure%20%28by%20ref%29))
  (bind _asbp_pipe (Utilities|Casting|CastToBP_Pipe OtherActor))
  (if (== OverlappedComponent (Variables|BP_Pipe_C|GetCollisionRight _asbp_pipe))
    (Development|PrintString "Left connected to Right")
    (elif (== OverlappedComponent (Variables|BP_Pipe_C|GetCollisionLeft _asbp_pipe))
      (Development|PrintString "Left connected to Left")
      (elif (== OverlappedComponent (Variables|BP_Pipe_C|GetCollisionBottom _asbp_pipe))
        (Development|PrintString "Left connected to Bottom")))))

(event EventBeginPlay
  (bind _staticmesh (Variables|Default|GetStaticMesh))
  (bind _relativerotation (Variables|/Script/Engine.SceneComponent|GetRelativeRotation _staticmesh))
  (|CallParentFunction)
  (Variables|Rotators|SetBaseRotation (Math|Rotator|MakeRotator (.roll _relativerotation) (.pitch _relativerotation) 0.0)))

(event Collision|EventActorBeginOverlap
  (params (OtherActor :type Actor%20Object%20Reference)))

(event EventTick
  (params (DeltaSeconds :type Float%20%28single-precision%29)))

(event EventInteract
  (bind _staticmesh (Variables|Default|GetStaticMesh))
  (bind _relativerotation (Variables|/Script/Engine.SceneComponent|GetRelativeRotation _staticmesh))
  (if (not (Variables|Booleans|GetbIsRotating))
    (Variables|Booleans|SetbIsRotating true)
    (Variables|Rotators|SetBaseRotation _relativerotation)
    (Variables|Rotators|SetEndRotation (Math|Rotator|CombineRotators _relativerotation (Math|Rotator|MakeRotator 0.0 0.0 9e+01)))
    (bind _piperotation (Timeline|PipeRotation PlayFromStart)
      (:Update
        (Transformation|SetRelativeRotation (Variables|Default|GetStaticMesh) (Math|Rotator|Lerp(Rotator) (Variables|Rotators|GetBaseRotation) (Variables|Rotators|GetEndRotation) _piperotation true) false false))
      (:Finished
        (Variables|Booleans|SetbIsRotating false)))))

(fn ConstructionScript
  (|CallParentFunction))