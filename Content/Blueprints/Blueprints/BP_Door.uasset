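; BP_Door is a key-locked swinging door that opens on Interact once PickUpKey has set HasKey.
; A DoorRotation timeline lerps the mesh's yaw to swing it open, and two close-box overlaps from the player reverse that timeline to shut it.
; When the timeline finishes, the resulting yaw sets IsDoorOpened, which gates further opening, and prints a status message.
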(event OnComponentBeginOverlap(CloseBox1)
  (params (OverlappedComponent :type Primitive%20Component%20Object%20Reference) (OtherActor :type Actor%20Object%20Reference) (OtherComp :type Primitive%20Component%20Object%20Reference) (OtherBodyIndex :type Integer) (bFromSweep :type Boolean) (SweepResult :type Hit%20Result%20Structure%20%28by%20ref%29))
  (if (== OtherActor (Variables|Default|GetPlayerCharacter))
    (bind _doorrotation (Timeline|DoorRotation Reverse)
      (:Update
        (Transformation|SetRelativeRotation (Variables|Default|GetStaticMesh1) (Math|Rotator|MakeRotator 0.0 0.0 (Math|Float|Lerp 0.0 -1.1e+02 _doorrotation)) false false))
      (:Finished
        (if (<= (.yaw (Variables|/Script/Engine.SceneComponent|GetRelativeRotation (Variables|Default|GetStaticMesh1))) -1.1e+02)
          (Variables|Default|SetisDoorOpened true)
          (Development|PrintString "door has been opened")
          (elif (>= (.yaw (Variables|/Script/Engine.SceneComponent|GetRelativeRotation (Variables|Default|GetStaticMesh1))) 0.0)
            (Variables|Default|SetisDoorOpened false)
            (Development|PrintString "door is closed")))))))

(event OnComponentBeginOverlap(CloseBox2)
  (params (OverlappedComponent :type Primitive%20Component%20Object%20Reference) (OtherActor :type Actor%20Object%20Reference) (OtherComp :type Primitive%20Component%20Object%20Reference) (OtherBodyIndex :type Integer) (bFromSweep :type Boolean) (SweepResult :type Hit%20Result%20Structure%20%28by%20ref%29))
  (if (== OtherActor (Variables|Default|GetPlayerCharacter))
    (bind _doorrotation (Timeline|DoorRotation Reverse)
      (:Update
        (Transformation|SetRelativeRotation (Variables|Default|GetStaticMesh1) (Math|Rotator|MakeRotator 0.0 0.0 (Math|Float|Lerp 0.0 -1.1e+02 _doorrotation)) false false))
      (:Finished
        (if (<= (.yaw (Variables|/Script/Engine.SceneComponent|GetRelativeRotation (Variables|Default|GetStaticMesh1))) -1.1e+02)
          (Variables|Default|SetisDoorOpened true)
          (Development|PrintString "door has been opened")
          (elif (>= (.yaw (Variables|/Script/Engine.SceneComponent|GetRelativeRotation (Variables|Default|GetStaticMesh1))) 0.0)
            (Variables|Default|SetisDoorOpened false)
            (Development|PrintString "door is closed")))))))

(event EventBeginPlay
  (|CallParentFunction) ; This node is disabled and will not be called.\nDrag off pins to build functionality.
)

(event Collision|EventActorBeginOverlap
  (params (OtherActor :type Actor%20Object%20Reference))
  (|CallParentFunction OtherActor))

(event EventTick
  (params (DeltaSeconds :type Float%20%28single-precision%29))
  (|CallParentFunction DeltaSeconds) ; This node is disabled and will not be called.\nDrag off pins to build functionality.
)

(event EventInteract
  (if (Variables|Default|GethasKey)
    (if (not (Variables|Default|GetisDoorOpened))
      (bind _doorrotation (Timeline|DoorRotation Play)
        (:Update
          (Transformation|SetRelativeRotation (Variables|Default|GetStaticMesh1) (Math|Rotator|MakeRotator 0.0 0.0 (Math|Float|Lerp 0.0 -1.1e+02 _doorrotation)) false false))
        (:Finished
          (if (<= (.yaw (Variables|/Script/Engine.SceneComponent|GetRelativeRotation (Variables|Default|GetStaticMesh1))) -1.1e+02)
            (Variables|Default|SetisDoorOpened true)
            (Development|PrintString "door has been opened")
            (elif (>= (.yaw (Variables|/Script/Engine.SceneComponent|GetRelativeRotation (Variables|Default|GetStaticMesh1))) 0.0)
              (Variables|Default|SetisDoorOpened false)
              (Development|PrintString "door is closed"))))))))

(event EventPickUpKey
  (Variables|Default|SethasKey true))

(fn ConstructionScript
  (|CallParentFunction))