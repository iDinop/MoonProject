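; BP_MoonlightReceiver is a puzzle sensor that charges while lit and activates linked objects when full.
; A looping timer raises or drains Charge based on the SetLit state and feeds it to a dynamic crescent material.
; At full charge it stops updating, so it stays latched, and calls ActivateMessage once through BPI_Puzzle on every implementer in ActivatableArray.
; The debug line draw is unconnected.
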(event Custom|ActivateElements
  (for _array_element (Variables|Actors|GetActivatableArray)
    (if (Utilities|DoesObjectImplementInterface _array_element "/Game/Blueprints/Interfaces/BPI_Puzzle.BPI_Puzzle_C")
      (Class|BPIPuzzle|Activate(Message) _array_element))))

(event Custom|SetLit
  (params (bNewLit :type Boolean))
  ;[0.15 0.15 0.15 0.5] Lit Function
  ;;[0 0 0] SetLit Event
  (Variables|Booleans|SetbIsLit bNewLit))

(event Custom|ChargeEvent
  (bind _checkinterval (Variables|Floats|GetCheckInterval))
  (bind _mid_sensor (Variables|Materials|GetMID_Sensor))
  ;[0.15 0.15 0.15 0.5] Lit Function
  (if (== (Variables|Floats|GetCharge) 1.0)
    (Utilities|FlowControl|DoOnce false
      (:Completed
        (Development|PrintString "Fully charged")
        (Variables|Booleans|SetbIsFullyCharged true)
        (CallFunction|ActivateElements)))
    (elif (Variables|Booleans|GetbIsLit)
      (bind _output_get (Variables|Floats|SetCharge (Math|Float|Clamp(Float) (+ (Variables|Floats|GetCharge) (* (Variables|Floats|GetChargeRate) _checkinterval)))))
      (Rendering|Material|SetScalarParameterValue _mid_sensor "Charge" _output_get :!class /Script/Engine.MaterialInstanceDynamic)
      (else
        (Variables|Floats|SetCharge (Math|Float|Clamp(Float) (- (Variables|Floats|GetCharge) (* (Variables|Floats|GetDischargeRate) _checkinterval))))
        (Rendering|Material|SetScalarParameterValue _mid_sensor "Charge" _output_get :!class /Script/Engine.MaterialInstanceDynamic)))))

(event EventBeginPlay
  ;[0.15 0.15 0.15 0.5] Lit Function
  (bind _returnvalue (Rendering|Material|CreateDynamicMaterialInstance (Variables|Default|GetMoonCrescent_Mesh) 0 "/Game/Materials/MI_SensorCrescent.MI_SensorCrescent" "None" :!class /Script/Engine.PrimitiveComponent))
  (Variables|Materials|SetMID_Sensor _returnvalue)
  (Utilities|Time|SetTimerbyEvent (delegate Custom|ChargeEvent) (Variables|Floats|GetCheckInterval) true))

(event EventTick
  (params (DeltaSeconds :type Float%20%28single-precision%29))
  ;[0.15 0.15 0.15 0.5] Draw Debug Line
)

(fn ConstructionScript)