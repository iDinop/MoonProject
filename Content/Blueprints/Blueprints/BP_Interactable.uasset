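; BP_Interactable is an interactable actor that shows a prompt widget when the player stands near it.
; BeginPlay caches the player's BP_FirstPersonCharacter, and the BoxCollision overlap events show or hide the Widget component when that character enters or leaves.
; Each overlap also prints a debug message; the file contains no interaction logic beyond this visibility toggle.
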(event OnComponentEndOverlap(BoxCollision)
  (params (OverlappedComponent :type Primitive%20Component%20Object%20Reference) (OtherActor :type Actor%20Object%20Reference) (OtherComp :type Primitive%20Component%20Object%20Reference) (OtherBodyIndex :type Integer))
  (if (== OtherActor (Variables|Default|GetPlayerCharacter))
    (Rendering|SetVisibility (Variables|Default|GetWidget) false false)
    (Development|PrintString "Exited Collision")))

(event OnComponentBeginOverlap(BoxCollision)
  (params (OverlappedComponent :type Primitive%20Component%20Object%20Reference) (OtherActor :type Actor%20Object%20Reference) (OtherComp :type Primitive%20Component%20Object%20Reference) (OtherBodyIndex :type Integer) (bFromSweep :type Boolean) (SweepResult :type Hit%20Result%20Structure%20%28by%20ref%29))
  (if (== OtherActor (Variables|Default|GetPlayerCharacter))
    (Rendering|SetVisibility (Variables|Default|GetWidget) true false)
    (Development|PrintString "Entered Collision")))

(event EventBeginPlay
  (bind _asbp_first_person_character (Utilities|Casting|CastToBP_FirstPersonCharacter (Game|GetPlayerCharacter 0)))
  (Variables|Default|SetPlayerCharacter _asbp_first_person_character))

(fn ConstructionScript)